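; GameManager runs the game's wave progression and score display.
; It spawns wave actors from the Waves array at its own transform, with IterateWave advancing the index until none remain.
; IterateScore adds a set increment to Score and refreshes ScoreText.
; FinishedWaves turns on auto-launch and fires every TS_FireworksLauncher; it runs after the last wave and also on BeginPlay, right after the first spawn.
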(event `self.ReceiveBeginPlay`
  (`self.SpawnWave`)
  (`self.UpdateTextWithScore`)
  (`self.FinishedWaves`))

(event `SpawnWave`
  (bind _returnvalue (`|SpawnActorFromClass` (`|GetArrayItem` (`self.Waves`) (`self.WavesIndex`)) (`self.GetTransform` self) "Undefined" "OverrideRootScale" null null))
  (set `self.CurrentWave` _returnvalue))

(event `IterateWave`
  (bind _wavesindex (`self.WavesIndex`))
  (`/Engine/EditorBlueprintResources/StandardMacros.IncrementInt` _wavesindex
    (:`  `
      (if (< _wavesindex (`KismetArrayLibrary.Array_Length` (`self.Waves`)))
        (`self.SpawnWave`)
        (else
          (`self.FinishedWaves`))))))

(event `IterateScore`
  (set `self.Score` (+ (`self.Score`) (`self.ScoreIterationAmount`)))
  (`self.UpdateTextWithScore`))

(event `UpdateTextWithScore`
  (`TextRenderComponent.K2_SetText` (`self.ScoreText`) (`KismetTextLibrary.Conv_IntToText` (`self.Score`))))

(event `FinishedWaves`
  (`KismetSystemLibrary.PrintString` "In finished waves")
  (bind _outactors (`GameplayStatics.GetAllActorsOfClass` "/Game/TS_Fireworks/Blueprints/TS_FireworksLauncher.TS_FireworksLauncher_C"))
  (for _array_element _outactors
    (set `/Game/TS_Fireworks/Blueprints/TS_FireworksLauncher.AutoLaunch` true _array_element)
    (`/Game/TS_Fireworks/Blueprints/TS_FireworksLauncher.LaunchTimedShell` _array_element)))

(fn `UserConstructionScript`)