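; Grabbable VR tennis racket for Vive that rumbles the holding hand when its head hits a Ball-tagged actor.
; Pickup, called by BP_MotionController, disables physics and snaps the racket to the attach component with a fixed grip offset; Drop detaches it and restores physics.
; StopVelocity zeroes mesh and head velocities and restores the rotation cached at BeginPlay.
; PickupAction and OnPickup only print debug strings.
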(event `self.ReceiveBeginPlay`
  (set `self.DefaultRotation` (`SceneComponent.K2_GetComponentRotation` (`self.StaticMeshComponent`))))

(event `/Game/VirtualRealityBP/Blueprints/PickupActorInterface.Pickup`
  (params (AttachTo :type "SceneComponent Object Reference"))
  (`PrimitiveComponent.SetSimulatePhysics` (`self.StaticMeshComponent`) false)
  (`SceneComponent.K2_AttachToComponent` (`self.K2_GetRootComponent`) AttachTo "None" "SnapToTarget" "SnapToTarget" "KeepWorld" false)
  (`SceneComponent.K2_SetRelativeLocationAndRotation` (`self.StaticMeshComponent`) (-50.0 -35.0 -35.0) (struct :`Pitch` 90.0 :`Yaw` 90.0) false false))

(event `/Game/VirtualRealityBP/Blueprints/PickupActorInterface.Drop`
  (`PrimitiveComponent.SetSimulatePhysics` (`self.StaticMeshComponent`) true)
  (`self.K2_DetachFromActor` "KeepWorld" "KeepWorld" "KeepWorld"))

(event `Stop Velocity`
  (bind _staticmeshcomponent (`self.StaticMeshComponent`))
  (bind _head (`self.Head`))
  (`PrimitiveComponent.SetAllPhysicsLinearVelocity` _staticmeshcomponent (0.0 0.0 0.0) false)
  (`PrimitiveComponent.SetAllPhysicsAngularVelocityInDegrees` _staticmeshcomponent (`KismetMathLibrary.Vector_Zero`) false)
  (`PrimitiveComponent.SetAllPhysicsLinearVelocity` _head (0.0 0.0 0.0) false)
  (`PrimitiveComponent.SetAllPhysicsAngularVelocityInDegrees` _head (`KismetMathLibrary.Vector_Zero`) false)
  (`SceneComponent.K2_SetWorldRotation` _staticmeshcomponent (`self.DefaultRotation`) false false))

(event `self.Head.OnComponentHit`
  (params (HitComponent :type "PrimitiveComponent Object Reference") (OtherActor :type "Actor Object Reference") (OtherComp :type "PrimitiveComponent Object Reference") (NormalImpulse :type "Vector Structure") (Hit :type "HitResult Structure (by ref)"))
  (if (and (`KismetArrayLibrary.Array_Contains` (`Actor.Tags` OtherActor) "Ball") (`self.IsBeingHeld`))
    (`/Game/VirtualRealityBP/Blueprints/BP_MotionController.RumbleController` (`self.HandHoldingYou`) 0.3)))

(event `PickupAction`
  (`KismetSystemLibrary.PrintString` "PickupAction child"))

(event `self.OnPickup`
  (`KismetSystemLibrary.PrintString` "On pickup Child"))

(fn `UserConstructionScript`)