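; Cube actor Blueprint that cycles through a list of colours each time its ChangeColour event fires.
; The construction script creates a dynamic material instance on the Cube and sets its Base_Color parameter to the first colour in the Colors array.
; ChangeColour advances ColorIndex, wrapping back to the start after the last entry, and applies that colour to the stored material instance.
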(event `ChangeColour`
  (if (< (`self.colorIndex`) (- (`KismetArrayLibrary.Array_Length` (`self.Colors`)) 1))
    (`/Engine/EditorBlueprintResources/StandardMacros.IncrementInt` (`self.colorIndex`)
      (:`  `
        _))
    (else
      (set `self.colorIndex` 0)))
  (`MaterialInstanceDynamic.SetVectorParameterValue` (`self.MaterialInstance`) "Base_Color" (`KismetMathLibrary.Conv_ColorToLinearColor` (`|GetArrayItem` (`self.Colors`) (`self.colorIndex`)))))

(event `self.ReceiveBeginPlay`)

(fn `UserConstructionScript`
  (bind _returnvalue (`PrimitiveComponent.CreateDynamicMaterialInstance` (`self.Cube`) 0 null "None"))
  (set `self.MaterialInstance` _returnvalue)
  (`MaterialInstanceDynamic.SetVectorParameterValue` _returnvalue "Base_Color" (`KismetMathLibrary.Conv_ColorToLinearColor` (`|GetArrayItem` (`self.Colors`)))))