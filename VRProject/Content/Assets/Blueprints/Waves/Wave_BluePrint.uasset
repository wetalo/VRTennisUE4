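; Wave actor that tracks remaining targets and advances the game to the next wave once they are gone.
; On BeginPlay it gathers every actor tagged "Target" in the level and stores the count, printing it for debugging.
; SubtractTarget decrements that count, and at zero calls IterateWave on the first GameManager found, then destroys the wave actor.
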(event `self.ReceiveBeginPlay`
  (`self.GetAllTargets`))

(event `GetAllTargets`
  (bind _outactors (`GameplayStatics.GetAllActorsWithTag` "Target"))
  (bind _output_get (set `self.Targets` _outactors))
  (bind _output_get_2 (set `self.numTargets` (`KismetArrayLibrary.Array_Length` _output_get)))
  (`KismetSystemLibrary.PrintString` (`KismetStringLibrary.Concat_StrStr` "Num Targets:" (`KismetStringLibrary.Conv_IntToString` _output_get_2))))

(event `self.ReceiveTick`
  (params (DeltaSeconds :type "Float (single-precision)")))

(event `SubtractTarget`
  (bind _numtargets (`self.numTargets`))
  (`/Engine/EditorBlueprintResources/StandardMacros.DecrementInt` _numtargets
    (:`  `
      (if (<= _numtargets 0)
        (bind _outactors (`GameplayStatics.GetAllActorsOfClass` "/Game/Assets/Blueprints/GameManager.GameManager_C"))
        (`/Game/Assets/Blueprints/GameManager.IterateWave` (`|GetArrayItem` _outactors))
        (`self.K2_DestroyActor`)))))

(fn `UserConstructionScript`)