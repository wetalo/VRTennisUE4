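; BallSpawner is an actor that launches Ball actors when the player presses the ShootBall input action.
; It enables input from the first player controller on BeginPlay.
; Each press spawns a Ball at the BallSpawnPoint component's world location and applies a fixed, mass-dependent impulse to its Sphere along that component's up vector.
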(event `self.ReceiveBeginPlay`
  (`self.EnableInput` (`GameplayStatics.GetPlayerController` 0)))

(event `InputAction|ShootBall`
  (params (Key :type "Key Structure"))
  (:`Pressed`
    (bind _returnvalue (`|SpawnActorFromClass` "/Game/Assets/Blueprints/Ball.Ball_C" (`KismetMathLibrary.Conv_VectorToTransform` (`SceneComponent.K2_GetComponentLocation` (`self.BallSpawnPoint`))) "Undefined" "OverrideRootScale" null null))
    (`PrimitiveComponent.AddImpulse` (`/Game/Assets/Blueprints/Ball.Sphere` _returnvalue) (* (`SceneComponent.GetUpVector` (`self.BallSpawnPoint`)) 4500.0) "None" false)))

(fn `UserConstructionScript`)